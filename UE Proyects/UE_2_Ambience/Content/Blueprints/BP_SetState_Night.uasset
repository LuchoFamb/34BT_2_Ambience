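; BP_SetState_Night is a trigger volume that switches the DayTime audio-style state group to Night while the player is inside it.
; Box begin overlap with the player character sets the state to Night, and end overlap sets it back to Day.
; The construction script sizes the box from the InBoxExtent variable, so each placed instance can be resized.
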(event `self.Box.OnComponentBeginOverlap`
  (params (OverlappedComponent :type "PrimitiveComponent Object Reference") (OtherActor :type "Actor Object Reference") (OtherComp :type "PrimitiveComponent Object Reference") (OtherBodyIndex :type Integer) (bFromSweep :type Boolean) (SweepResult :type "HitResult Structure (by ref)"))
  ;[1 1 1] Set Night State
  (if (== OtherActor (`GameplayStatics.GetPlayerCharacter` 0))
    (`AkGameplayStatics.SetState` "/Game/Audio/States/Default_Work_Unit/Environmental/DayTime/DayTime-Night.DayTime-Night" "DayTime" "Night")))

(event `self.Box.OnComponentEndOverlap`
  (params (OverlappedComponent :type "PrimitiveComponent Object Reference") (OtherActor :type "Actor Object Reference") (OtherComp :type "PrimitiveComponent Object Reference") (OtherBodyIndex :type Integer))
  ;[1 1 1] Set Night State
  (if (== (`GameplayStatics.GetPlayerCharacter` 0) OtherActor)
    (`AkGameplayStatics.SetState` "/Game/Audio/States/Default_Work_Unit/Environmental/DayTime/DayTime-Day.DayTime-Day" "DayTime" "Day")))

(fn `UserConstructionScript`
  (`BoxComponent.SetBoxExtent` (`self.Box`) (`self.In Box Extent`) true))