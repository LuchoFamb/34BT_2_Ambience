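; Trigger box actor that alternates between two Wwise states, A and B, as the player passes through it.
; Each overlap begun by player character 0 advances a FlipFlop, which calls SetState with the A or B state value, group and name, starting with A.
; The construction script sizes the box from the InBoxExtent variable.
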(event `self.Box.OnComponentBeginOverlap`
  (params (OverlappedComponent :type "PrimitiveComponent Object Reference") (OtherActor :type "Actor Object Reference") (OtherComp :type "PrimitiveComponent Object Reference") (OtherBodyIndex :type Integer) (bFromSweep :type Boolean) (SweepResult :type "HitResult Structure (by ref)"))
  (if (== OtherActor (`GameplayStatics.GetPlayerCharacter` 0))
    (`/Engine/EditorBlueprintResources/StandardMacros.FlipFlop`
      (:`A`
        (`AkGameplayStatics.SetState` (`self.State Value A`) (`self.State Group A`) (`self.State A`)))
      (:`B`
        (`AkGameplayStatics.SetState` (`self.State Value B`) (`self.State Group B`) (`self.State B`))))))

(fn `UserConstructionScript`
  (`BoxComponent.SetBoxExtent` (`self.Box`) (`self.In Box Extent`) true))