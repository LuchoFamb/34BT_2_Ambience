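; BP_Thunder_Trigger is a sphere trigger that drives Wwise weather audio from the player's position.
; Overlap events set the Weather state to Rain when the player enters and NoRain when they leave or another actor enters.
; Every tick it maps player height to the RainIntensity RTPC, posts the Environmental_Weather event and prints debug values.
; The construction script applies the configurable sphere radius.
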(event `self.ReceiveTick`
  (params (DeltaSeconds :type "Float (single-precision)"))
  ;[1 1 1] Set RTPC_RainIntensity on Tick
  (bind _output_get (set `self.PlayerHeight` (`KismetMathLibrary.MapRangeClamped` (.z (`self.K2_GetActorLocation` (`GameplayStatics.GetPlayerCharacter` 0))) (`self.Start Height`) (`self.End Height`) 0.0 100.0)))
  (`AkGameplayStatics.SetRTPCValue` "/Game/Audio/Game_Parameters/Default_Work_Unit/RTPC_RainIntensity.RTPC_RainIntensity" _output_get 0 null "RTPC_RainIntensity")
  (`AkGameplayStatics.PostEvent` :`AkEvent` "/Game/Audio/Events/Default_Work_Unit/Environmental_Weather.Environmental_Weather" :`EventName` "Environmental_Weather")
  ;[1 1 1] Debug Print Text
  (bind _value (`AkGameplayStatics.GetRTPCValue` "/Game/Audio/Game_Parameters/Default_Work_Unit/RTPC_RainIntensity.RTPC_RainIntensity" 0 "GameObject" null "RTPC_RainIntensity"))
  (`KismetSystemLibrary.PrintText` (`|FormatText` "Z Player; {Z}    RTPC Value; {RTPC}" (`self.PlayerHeight`) _value) true true (struct :`G` 0.66 :`B` 1.0 :`A` 1.0) 0.2))

(event `self.Sphere.OnComponentBeginOverlap`
  (params (OverlappedComponent :type "PrimitiveComponent Object Reference") (OtherActor :type "Actor Object Reference") (OtherComp :type "PrimitiveComponent Object Reference") (OtherBodyIndex :type Integer) (bFromSweep :type Boolean) (SweepResult :type "HitResult Structure (by ref)"))
  ;[1 1 1] Sphere On Component Begin Overlap --> Set State Rain
  (if (== OtherActor (`GameplayStatics.GetPlayerCharacter` 0))
    (`AkGameplayStatics.SetState` "/Game/Audio/States/Default_Work_Unit/Environmental/Weather/Weather-Rain.Weather-Rain" "Weather" "Rain")
    (else
      (`AkGameplayStatics.SetState` "/Game/Audio/States/Default_Work_Unit/Environmental/Weather/Weather-NoRain.Weather-NoRain" "Weather" "NoRain" :!label _label))))

(event `self.Sphere.OnComponentEndOverlap`
  (params (OverlappedComponent :type "PrimitiveComponent Object Reference") (OtherActor :type "Actor Object Reference") (OtherComp :type "PrimitiveComponent Object Reference") (OtherBodyIndex :type Integer))
  ;[1 1 1] Sphere On Component Begin Overlap --> Set State Rain
  (if (== (`GameplayStatics.GetPlayerCharacter` 0) OtherActor)
    (goto _label)))

(fn `UserConstructionScript`
  (`SphereComponent.SetSphereRadius` (`self.Sphere`) (`self.In Sphere Radius`) true))